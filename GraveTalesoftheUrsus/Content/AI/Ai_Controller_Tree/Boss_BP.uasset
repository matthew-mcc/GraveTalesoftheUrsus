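; Boss pawn Blueprint that prototypes a hand-built behavior tree to chase the player based on health.
; Helper functions test three health bands out of 1000, while Sequence and Selector functions imitate composite nodes with AND/OR results.
; Tick feeds the above-66% check through Sequence into MoveToPlayer, which runs AI MoveTo toward the player when passed.
; The middle-band branch is disconnected, and Selector and the lowest-band check are unused.
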(event `self.ReceiveTick`
  (params (DeltaSeconds :type "Float (single-precision)"))
  (bind _out1 (`self.Sequence` (stale _pass_fail)))
  (`|ExecutionSequence`
    (:`then_0`
      (bind _pass_fail (`self.Health > 66%`)))
    (:`then_1`
      (`self.MoveToPlayer` _out1))))

(event `MoveToPlayer`
  (params (`Previous Pass` :type Boolean))
  (if `Previous Pass`
    (`|AIMoveTo` self (0.0 0.0 0.0) (`GameplayStatics.GetPlayerCharacter` 0) 150.0)))

(fn `66% >= Health > 33%`
  (returns (`Pass/Fail` :type Boolean))
  (return (and (<= (/ (`KismetMathLibrary.Conv_IntToDouble` (`self.Health Points`)) 1000.0) 0.66) (> (/ (`KismetMathLibrary.Conv_IntToDouble` (`self.Health Points`)) 1000.0) 0.33))))

(fn `Health <= 33%`
  (returns (`Pass/Fail` :type Boolean))
  (return (<= (/ (`KismetMathLibrary.Conv_IntToDouble` (`self.Health Points`)) 1000.0) 0.33)))

(fn `Health > 66%`
  (returns (`Pass/Fail` :type Boolean))
  (return (> (/ (`KismetMathLibrary.Conv_IntToDouble` (`self.Health Points`)) 1000.0) 0.66)))

(fn `Selector`
  (params (In1 :type Boolean) (In2 :type Boolean) (In3 :type Boolean) (In4 :type Boolean) (In5 :type Boolean))
  (returns (Out1 :type Boolean) (Out2 :type Boolean) (Out3 :type Boolean) (Out4 :type Boolean) (Out5 :type Boolean) (`Pass/Fail` :type Boolean))
  (locals (Child1 :type Boolean :default false) (Child2 :type Boolean :default false) (Child3 :type Boolean :default false) (Child4 :type Boolean :default false) (Child5 :type Boolean :default false))
  (bind _output_get (set `local.Child1` In1))
  (bind _output_get_2 (set `local.Child2` In2))
  (bind _output_get_3 (set `local.Child3` In3))
  (bind _output_get_4 (set `local.Child4` In4))
  (bind _output_get_5 (set `local.Child5` In5))
  (return _output_get _output_get_2 _output_get_3 _output_get_4 _output_get_5 (or (`local.Child1`) (`local.Child2`) (`local.Child3`) (`local.Child4`) (`local.Child5`))))

(fn `Sequence`
  (params (In1 :type Boolean) (In2 :type Boolean) (In3 :type Boolean) (In4 :type Boolean) (In5 :type Boolean))
  (returns (Out1 :type Boolean) (Out2 :type Boolean) (Out3 :type Boolean) (Out4 :type Boolean) (Out5 :type Boolean) (`Pass/Fail` :type Boolean))
  (locals (Child1 :type Boolean :default true) (Child2 :type Boolean :default true) (Child3 :type Boolean :default true) (Child4 :type Boolean :default true) (Child5 :type Boolean :default true))
  (bind _output_get (set `local.Child1` In1))
  (bind _output_get_2 (set `local.Child2` In2))
  (bind _output_get_3 (set `local.Child3` In3))
  (bind _output_get_4 (set `local.Child4` In4))
  (bind _output_get_5 (set `local.Child5` In5))
  (return _output_get _output_get_2 _output_get_3 _output_get_4 _output_get_5 (and (`local.Child1`) (`local.Child2`) (`local.Child3`) (`local.Child4`) (`local.Child5`))))

(fn `UserConstructionScript`)